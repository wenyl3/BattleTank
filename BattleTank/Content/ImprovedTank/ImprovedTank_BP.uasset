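; ImprovedTank_BP is a player-controllable tank pawn that wires its aiming and movement components to input.
; BeginPlay hands the barrel and turret to TankAiming and both tracks to TankMovement.
; Movement and turn axes pass intents to TankMovement, while aim axes rotate an azimuth gimbal and spring arm, scaled by frame time.
; The Fire action calls Fire, whose logic is not defined in these graphs.
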(event `self.ReceiveBeginPlay`
  (`TankAimingComponent.Initialise` (`self.TankAiming`) (`self.Barrel`) (`self.Turret`))
  (`TankMovementComponent.Initialise` (`self.TankMovement`) (`self.LeftTrack`) (`self.RightTrack`)))

(event `InputAxis|AimElevation`
  (params (AxisValue :type "Float (single-precision)"))
  ;[1 1 1] InputBinding
  (`SceneComponent.K2_AddLocalRotation` (`self.SpringArm`) (`KismetMathLibrary.MakeRotator` 0.0 (* AxisValue (`GameplayStatics.GetWorldDeltaSeconds`) 100.0)) false false))

(event `InputAxis|ForwardMovement`
  (params (AxisValue :type "Float (single-precision)"))
  ;[1 1 1] MovementInputBinding
  (`TankMovementComponent.IntendMoveForward` (`self.TankMovement`) AxisValue))

(event `InputAxis|BackwardMovement`
  (params (AxisValue :type "Float (single-precision)"))
  ;[1 1 1] MovementInputBinding
  (`TankMovementComponent.IntendMoveBackward` (`self.TankMovement`) AxisValue))

(event `InputAxis|AimAzimuth`
  (params (AxisValue :type "Float (single-precision)"))
  ;[1 1 1] InputBinding
  (`SceneComponent.K2_AddLocalRotation` (`self.AzimuthGimble`) (`KismetMathLibrary.MakeRotator` 0.0 0.0 (* AxisValue (`GameplayStatics.GetWorldDeltaSeconds`) 100.0)) false false))

(event `InputAxis|TurnLeft`
  (params (AxisValue :type "Float (single-precision)"))
  ;[1 1 1] MovementInputBinding
  (`TankMovementComponent.IntendTurnLeft` (`self.TankMovement`) AxisValue))

(event `InputAxis|TurnRight`
  (params (AxisValue :type "Float (single-precision)"))
  ;[1 1 1] MovementInputBinding
  (`TankMovementComponent.IntendTurnRight` (`self.TankMovement`) AxisValue))

(event `InputAction|Fire`
  (params (Key :type "Key Structure"))
  ;[1 1 1] InputBinding
  (:`Pressed`
    (`self.Fire`)))

(fn `UserConstructionScript`)